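; PlayerController_Pedro is a player controller that handles pausing and sets up camera pitch limits and input mode.
; On BeginPlay it clamps the camera manager's vertical view range and switches to game-only input.
; Pressing Pause plays a UI sound, pauses the game, adds a new WBP_Pause widget to the viewport, shows the mouse cursor and switches to UI-only input.
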(event `InputAction|Pause`
  (params (Key :type "Key Structure"))
  (bind _returnvalue (`GameplayStatics.GetPlayerController` 0))
  (:`Pressed`
    (`GameplayStatics.SpawnSound2D` "/Game/Sounds/UI/Hovered/Hovered_sound.Hovered_sound" 1.0 1.0 0.0 null)
    (`GameplayStatics.SetGamePaused` true)
    (bind _returnvalue_2 (`|CreateWidget` "/Game/Blueprints/UI/WBP_Pause.WBP_Pause_C"))
    (bind _output_get (set `self.PauseMenu` _returnvalue_2))
    (`UserWidget.AddToViewport` _output_get 0)
    (set `PlayerController.bShowMouseCursor` true _returnvalue)
    (`WidgetBlueprintLibrary.SetInputMode_UIOnlyEx` _returnvalue null)))

(event `self.ReceiveBeginPlay`
  (bind _playercameramanager (`self.PlayerCameraManager`))
  (set `PlayerCameraManager.ViewPitchMin` -65.0 _playercameramanager)
  (set `PlayerCameraManager.ViewPitchMax` 10.0 _playercameramanager)
  (`WidgetBlueprintLibrary.SetInputMode_GameOnly` (`GameplayStatics.GetPlayerController` 0)))

(fn `UserConstructionScript`)