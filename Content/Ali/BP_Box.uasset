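; Wooden box actor that the Pedro player character interacts with, tracking what lies beneath it.
; A sphere overlap toggles Pedro's trace message and the BoxToBox flag, which selects the Tick downward trace from PointToFall.
; When set, the trace updates Pedro's BoxFloor1; otherwise a shorter trace attaches and snaps WoodBox to components tagged "overBox".
; Push capsule events are empty, physics experiments are disconnected, and debug prints and persistent trace drawing remain.
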(event `self.Capsule3.OnComponentBeginOverlap`
  (params (OverlappedComponent :type "PrimitiveComponent Object Reference") (OtherActor :type "Actor Object Reference") (OtherComp :type "PrimitiveComponent Object Reference") (OtherBodyIndex :type Integer) (bFromSweep :type Boolean) (SweepResult :type "HitResult Structure (by ref)"))
  ;[1 1 1] Capsules where you should position yourself to push the box
)

(event `self.Capsule2.OnComponentBeginOverlap`
  (params (OverlappedComponent :type "PrimitiveComponent Object Reference") (OtherActor :type "Actor Object Reference") (OtherComp :type "PrimitiveComponent Object Reference") (OtherBodyIndex :type Integer) (bFromSweep :type Boolean) (SweepResult :type "HitResult Structure (by ref)"))
  ;[1 1 1] Capsules where you should position yourself to push the box
)

(event `self.Capsule2.OnComponentEndOverlap`
  (params (OverlappedComponent :type "PrimitiveComponent Object Reference") (OtherActor :type "Actor Object Reference") (OtherComp :type "PrimitiveComponent Object Reference") (OtherBodyIndex :type Integer))
  ;[1 1 1] Capsules where you should position yourself to push the box
)

(event `self.Capsule3.OnComponentEndOverlap`
  (params (OverlappedComponent :type "PrimitiveComponent Object Reference") (OtherActor :type "Actor Object Reference") (OtherComp :type "PrimitiveComponent Object Reference") (OtherBodyIndex :type Integer))
  ;[1 1 1] Capsules where you should position yourself to push the box
)

(event `self.Capsule1.OnComponentBeginOverlap`
  (params (OverlappedComponent :type "PrimitiveComponent Object Reference") (OtherActor :type "Actor Object Reference") (OtherComp :type "PrimitiveComponent Object Reference") (OtherBodyIndex :type Integer) (bFromSweep :type Boolean) (SweepResult :type "HitResult Structure (by ref)"))
  ;[1 1 1] Capsules where you should position yourself to push the box
)

(event `self.Capsule.OnComponentEndOverlap`
  (params (OverlappedComponent :type "PrimitiveComponent Object Reference") (OtherActor :type "Actor Object Reference") (OtherComp :type "PrimitiveComponent Object Reference") (OtherBodyIndex :type Integer))
  ;[1 1 1] Capsules where you should position yourself to push the box
)

(event `self.Capsule.OnComponentBeginOverlap`
  (params (OverlappedComponent :type "PrimitiveComponent Object Reference") (OtherActor :type "Actor Object Reference") (OtherComp :type "PrimitiveComponent Object Reference") (OtherBodyIndex :type Integer) (bFromSweep :type Boolean) (SweepResult :type "HitResult Structure (by ref)"))
  ;[1 1 1] Capsules where you should position yourself to push the box
)

(event `self.Capsule1.OnComponentEndOverlap`
  (params (OverlappedComponent :type "PrimitiveComponent Object Reference") (OtherActor :type "Actor Object Reference") (OtherComp :type "PrimitiveComponent Object Reference") (OtherBodyIndex :type Integer))
  ;[1 1 1] Capsules where you should position yourself to push the box
)

(event `self.ReceiveBeginPlay`
  ;[1 1 1] Cast to Pedro_CharacterJump
)

(event `self.ReceiveTick`
  (params (DeltaSeconds :type "Float (single-precision)"))
  (bind _pointtofall (`self.PointToFall`))
  (bind _returnvalue (`SceneComponent.K2_GetComponentLocation` _pointtofall))
  (if (`self.BoxToBox`)
    (bind (_outhit _returnvalue_2) (`KismetSystemLibrary.LineTraceSingle` :`Start` _returnvalue :`End` (+ _returnvalue (* (`KismetMathLibrary.GetUpVector` (`SceneComponent.K2_GetComponentRotation` _pointtofall)) -50.0)) :`TraceChannel` "TraceTypeQuery1" :`DrawDebugType` "Persistent"))
    (if _returnvalue_2
      (bind _asbp_pedro_character_jump (cast `/Game/Ali/BP_PedroCharacterJump` (`GameplayStatics.GetPlayerCharacter` 0)))
      (bind _output_get (set `self.Pedrito` _asbp_pedro_character_jump))
      (set `/Game/Ali/BP_PedroCharacterJump.BoxFloor1` true _output_get)
      (else
        (`KismetSystemLibrary.PrintString` "No")
        (bind _asbp_pedro_character_jump_2 (cast `/Game/Ali/BP_PedroCharacterJump` (`GameplayStatics.GetPlayerCharacter` 0))
          (:`then`
            (bind _output_get_2 (set `self.Pedrito` _asbp_pedro_character_jump_2))
            (bind _output_get_3 (set `/Game/Ali/BP_PedroCharacterJump.BoxFloor1` false _output_get_2))
            (if _output_get_3
              (`KismetSystemLibrary.PrintString` "MAMO")
              (else
                (`KismetSystemLibrary.PrintString` "EN TEORÍA CHI"))))
          (:`CastFailed`
            (`KismetSystemLibrary.PrintString` "FALLO CAST SOLTAR CAJA")))))
    (else
      (bind (_outhit_2 _returnvalue_3) (`KismetSystemLibrary.LineTraceSingle` :`Start` _returnvalue :`End` (+ _returnvalue (* (`KismetMathLibrary.GetUpVector` (`SceneComponent.K2_GetComponentRotation` _pointtofall)) -20.0)) :`TraceChannel` "TraceTypeQuery1" :`DrawDebugType` "Persistent"))
      (if _returnvalue_3
        (if (`ActorComponent.ComponentHasTag` (`.HitComponent` (`GameplayStatics.BreakHitResult` _outhit_2)) "overBox")
          (`KismetSystemLibrary.PrintString` "TOCANDO CAJA" true true (struct :`G` 0.66 :`B` 1.0 :`A` 1.0) 10.0)
          (`SceneComponent.K2_AttachToComponent` (`self.WoodBox`) (`.HitComponent` (`GameplayStatics.BreakHitResult` _outhit_2)) "None" "KeepWorld" "KeepRelative" "KeepWorld" true)
          (`SceneComponent.K2_SetWorldLocation` (`self.WoodBox`) (`SceneComponent.K2_GetComponentLocation` (`.HitComponent` (`GameplayStatics.BreakHitResult` _outhit_2))) false false))))))

(event `self.Sphere4.OnComponentBeginOverlap`
  (params (OverlappedComponent :type "PrimitiveComponent Object Reference") (OtherActor :type "Actor Object Reference") (OtherComp :type "PrimitiveComponent Object Reference") (OtherBodyIndex :type Integer) (bFromSweep :type Boolean) (SweepResult :type "HitResult Structure (by ref)"))
  ;[1 1 1] Sphere Overlap to Cast Pedro & detect her tag
  (bind _asbp_pedro_character_jump (cast `/Game/Ali/BP_PedroCharacterJump` OtherActor))
  (bind _output_get (set `self.Pedro` _asbp_pedro_character_jump))
  (message `/Game/Blueprints/Interfaces/BI_ActionInterface.Trace` _output_get)
  (`KismetSystemLibrary.PrintString` "trace")
  (set `self.BoxToBox` true))

(event `self.Sphere4.OnComponentEndOverlap`
  (params (OverlappedComponent :type "PrimitiveComponent Object Reference") (OtherActor :type "Actor Object Reference") (OtherComp :type "PrimitiveComponent Object Reference") (OtherBodyIndex :type Integer))
  ;[1 1 1] Sphere Overlap to Cast Pedro & detect her tag
  (bind _asbp_pedro_character_jump (cast `/Game/Ali/BP_PedroCharacterJump` OtherActor))
  (message `/Game/Blueprints/Interfaces/BI_ActionInterface.NoTrace` _asbp_pedro_character_jump)
  (`KismetSystemLibrary.PrintString` "No trace")
  (set `self.BoxToBox` false))

(event `self.FallBox1.OnComponentBeginOverlap`
  (params (OverlappedComponent :type "PrimitiveComponent Object Reference") (OtherActor :type "Actor Object Reference") (OtherComp :type "PrimitiveComponent Object Reference") (OtherBodyIndex :type Integer) (bFromSweep :type Boolean) (SweepResult :type "HitResult Structure (by ref)")))

(event `self.FallBox1.OnComponentEndOverlap`
  (params (OverlappedComponent :type "PrimitiveComponent Object Reference") (OtherActor :type "Actor Object Reference") (OtherComp :type "PrimitiveComponent Object Reference") (OtherBodyIndex :type Integer)))

(event `self.Base.OnComponentBeginOverlap`
  (params (OverlappedComponent :type "PrimitiveComponent Object Reference") (OtherActor :type "Actor Object Reference") (OtherComp :type "PrimitiveComponent Object Reference") (OtherBodyIndex :type Integer) (bFromSweep :type Boolean) (SweepResult :type "HitResult Structure (by ref)")))

(fn `UserConstructionScript`)