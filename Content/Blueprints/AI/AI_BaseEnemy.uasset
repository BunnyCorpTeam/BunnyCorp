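; Base enemy AI that starts one of two looping patrol behaviours on BeginPlay, selected by its AIState.
; Patrol uses AIMoveTo to shuttle between the first two Targets with a pause at each, and has no failure handling.
; Patrol2 moves to a random Target and repeats after success or failure; its inclusive random maximum can index past the array.
; Unconnected nodes would spawn a TargetPoint at its position and add it to Targets.
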(event `self.ReceiveBeginPlay`
  (switch `/Game/Blueprints/AI/EAIState` (`self.AIState`)
    (:`NewEnumerator2`
      (`self.Patrol`))
    (:`NewEnumerator3`
      (`self.Patrol2`))))

(event `Patrol`
  (`|AIMoveTo` self (0.0 0.0 0.0) (`|GetArrayItem` (`self.Targets`))
    (:`OnSuccess`
      (`KismetSystemLibrary.Delay` 2.0)
      (`|AIMoveTo` self (0.0 0.0 0.0) (`|GetArrayItem` (`self.Targets`) 1)
        (:`OnSuccess`
          (`KismetSystemLibrary.Delay` 2.0)
          (`self.Patrol`))))))

(event `Patrol2`
  (bind _targets (`self.Targets`))
  (`|AIMoveTo` self (0.0 0.0 0.0) (`|GetArrayItem` _targets (`KismetMathLibrary.RandomIntegerInRange` 0 (`KismetArrayLibrary.Array_Length` _targets)))
    (:`OnSuccess`
      _)
    (:`OnFail`
      _))
  (`KismetSystemLibrary.Delay` 1.0)
  (`self.Patrol2`))

(fn `UserConstructionScript`)