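; BP_CarrotPick is a carrot pickup actor that runs a timing minigame to harvest the carrot.
; Sphere overlap caches Enriqueta and toggles the text prompt.
; Interact runs once, starting a delay-looped ping-pong counter, randomizing a target window and calling DeactivateMovementMessage on her.
; Minijuego checks the counter against that window: success destroys the carrot mesh and calls ReactivateMovementMessage, while feedback is only debug prints.
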(event `/Game/Blueprints/Actors/InteractInterface.Interact`
  (`/Engine/EditorBlueprintResources/StandardMacros.DoOnce` false
    (:`Completed`
      (`self.Contador`)
      (`self.RangoCorrecto`)
      (message `/Game/Blueprints/Actors/BI_InteractInterface.DeactivateMovement` (`self.Enriqueta`)))))

(event `Contador`
  (if (not (`self.Complete?`))
    (`KismetSystemLibrary.Delay` (`self.Speed`) :!label _label)
    (if (`self.Complete?`)
      _
      (elif (`self.1 A 10`)
        (`/Engine/EditorBlueprintResources/StandardMacros.IncrementInt` (`self.ElContador`)
          (:`  `
            (if (>= (`self.ElContador`) (`self.MaxContador`))
              (set `self.1 A 10` false)
              (goto _label)
              (else
                (`KismetSystemLibrary.PrintString` (`KismetStringLibrary.Conv_IntToString` (`self.ElContador`)))
                (goto _label)))))
        (else
          (`/Engine/EditorBlueprintResources/StandardMacros.DecrementInt` (`self.ElContador`)
            (:`  `
              (if (<= (`self.ElContador`) (`self.MinContador`))
                (set `self.1 A 10` true)
                (goto _label)
                (else
                  (`KismetSystemLibrary.PrintString` (`KismetStringLibrary.Conv_IntToString` (`self.ElContador`)))
                  (goto _label))))))))))

(event `/Game/Blueprints/Actors/InteractInterface.Minijuego`
  (if (>= (`self.ElContador`) (`self.MinCorrecto`))
    (if (<= (`self.ElContador`) (`self.MaxCorrecto`))
      (set `self.Complete?` true)
      (`ActorComponent.K2_DestroyComponent` (`self.SM_Carrot`))
      (`KismetSystemLibrary.PrintString` "Correcto" true true (struct :`R` 0.13916 :`G` 1.0 :`A` 1.0))
      (message `/Game/Blueprints/Actors/BI_InteractInterface.ReactivateMovement` (`self.Enriqueta`))
      (else
        (`KismetSystemLibrary.PrintString` "ERROR" true true (struct :`R` 1.0 :`G` 0.030993 :`A` 1.0))))
    (else
      (`KismetSystemLibrary.PrintString` "ERROR" true true (struct :`R` 1.0 :`G` 0.030993 :`A` 1.0)))))

(event `RangoCorrecto`
  (set `self.LimiteRango` (- (`self.MaxContador`) (`self.RangoError`)))
  (bind _output_get (set `self.MinCorrecto` (`KismetMathLibrary.RandomIntegerInRange` (`self.MinContador`) (`self.LimiteRango`))))
  (bind _output_get_2 (set `self.MaxCorrecto` (+ (`self.MinCorrecto`) (`self.RangoError`))))
  (`KismetSystemLibrary.PrintString` (`KismetStringLibrary.Concat_StrStr` "Minimo: " (`KismetStringLibrary.Conv_IntToString` _output_get) " " "Máximo: " (`KismetStringLibrary.Conv_IntToString` _output_get_2)) true true (struct :`G` 1.0 :`B` 0.023826 :`A` 1.0) 100.0))

(event `self.Sphere.OnComponentBeginOverlap`
  (params (OverlappedComponent :type "PrimitiveComponent Object Reference") (OtherActor :type "Actor Object Reference") (OtherComp :type "PrimitiveComponent Object Reference") (OtherBodyIndex :type Integer) (bFromSweep :type Boolean) (SweepResult :type "HitResult Structure (by ref)"))
  (bind _asbp_enriqueta_character (cast `/Game/Blueprints/Character/BP_EnriquetaCharacter` OtherActor))
  (set `self.Enriqueta` _asbp_enriqueta_character)
  (`SceneComponent.SetHiddenInGame` (`self.TextRender`) false false))

(event `self.Sphere.OnComponentEndOverlap`
  (params (OverlappedComponent :type "PrimitiveComponent Object Reference") (OtherActor :type "Actor Object Reference") (OtherComp :type "PrimitiveComponent Object Reference") (OtherBodyIndex :type Integer))
  (cast `/Game/Blueprints/Character/BP_EnriquetaCharacter` OtherActor)
  (`SceneComponent.SetHiddenInGame` (`self.TextRender`) true false))

(fn `UserConstructionScript`)